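; Behavior tree task that picks a random wander destination for a ChibiCharacter AI.
; On execute it writes the pawn's current location to the WanderOrigin blackboard key and sets walk speed to WanderSpeed.
; A reachable point within WanderRadius becomes WanderDestination and the task succeeds; otherwise the origin is written and it fails.
; A failed character cast stops execution without finishing the task.
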(event `self.ReceiveExecuteAI`
  (params (OwnerController :type "AIController Object Reference") (ControlledPawn :type "Pawn Object Reference"))
  (bind _wanderdestination (`self.WanderDestination`))
  (bind _returnvalue (`BTFunctionLibrary.GetBlackboardValueAsVector` (`self.WanderOrigin`)))
  (bind (_randomlocation _returnvalue_2) (`NavigationSystemV1.K2_GetRandomReachablePointInRadius` _returnvalue (`self.WanderRadius`) null null))
  (`BTFunctionLibrary.SetBlackboardValueAsVector` (`self.WanderOrigin`) (`Actor.K2_GetActorLocation` ControlledPawn))
  (bind _aschibi_character (cast `ChibiCharacter` ControlledPawn))
  (set `CharacterMovementComponent.MaxWalkSpeed` (`self.WanderSpeed`) (`Character.CharacterMovement` _aschibi_character))
  (if _returnvalue_2
    (`BTFunctionLibrary.SetBlackboardValueAsVector` _wanderdestination _randomlocation)
    (`self.FinishExecute` true)
    (else
      (`BTFunctionLibrary.SetBlackboardValueAsVector` _wanderdestination _returnvalue)
      (`self.FinishExecute` false))))